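; Main character Blueprint that shows an on-screen widget reflecting whether the player holds a torch.
; BeginPlay adds the not-holding widget to the viewport.
; E and G run identical logic: after a short delay they read HoldingTorch, print a debug message, remove all widgets and create the matching one.
; HoldingTorch is only read here, never set.
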(event EventBeginPlay
  (bind _returnvalue (UserInterface|CreateWidget "/Game/Hud/Game_Hud/BP_IsNotHoldingTorch.BP_IsNotHoldingTorch_C"))
  (UserInterface|Viewport|AddtoViewport _returnvalue 0))

(event Collision|EventActorBeginOverlap
  (params (OtherActor :type Actor%20Object%20Reference)))

(event EventTick
  (params (DeltaSeconds :type Float%20%28single-precision%29)))

(event Input|KeyboardEvents|E
  (params (Key :type Key%20Structure :default "None"))
  (:Pressed
    (Utilities|FlowControl|Delay 0.1)
    (if (Variables|Default|GetbHoldingTorch)
      (Development|PrintText "Torch true")
      (Viewport|RemoveAllWidgets)
      (bind _returnvalue (UserInterface|CreateWidget "/Game/Hud/Game_Hud/BP_IsHoldingTorch.BP_IsHoldingTorch_C"))
      (UserInterface|Viewport|AddtoViewport _returnvalue 0)
      (else
        (Development|PrintText "Torch false")
        (Viewport|RemoveAllWidgets)
        (bind _returnvalue_2 (UserInterface|CreateWidget "/Game/Hud/Game_Hud/BP_IsNotHoldingTorch.BP_IsNotHoldingTorch_C"))
        (UserInterface|Viewport|AddtoViewport _returnvalue_2 0)))))

(event Input|KeyboardEvents|G
  (params (Key :type Key%20Structure :default "None"))
  (:Pressed
    (Utilities|FlowControl|Delay 0.1)
    (if (Variables|Default|GetbHoldingTorch)
      (Development|PrintText "Torch true")
      (Viewport|RemoveAllWidgets)
      (bind _returnvalue (UserInterface|CreateWidget "/Game/Hud/Game_Hud/BP_IsHoldingTorch.BP_IsHoldingTorch_C"))
      (UserInterface|Viewport|AddtoViewport _returnvalue 0)
      (else
        (Development|PrintText "Torch false")
        (Viewport|RemoveAllWidgets)
        (bind _returnvalue_2 (UserInterface|CreateWidget "/Game/Hud/Game_Hud/BP_IsNotHoldingTorch.BP_IsNotHoldingTorch_C"))
        (UserInterface|Viewport|AddtoViewport _returnvalue_2 0)))))

(fn ConstructionScript)